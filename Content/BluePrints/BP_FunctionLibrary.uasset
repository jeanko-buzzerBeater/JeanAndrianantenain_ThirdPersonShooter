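; Blueprint function library that provides RNGVector, a helper for randomizing a vector.
; It multiplies each axis of the input vector by its own random float drawn between the given minimum and maximum.
; Because each axis rolls independently, both direction and length can change, and the scaled components return as three separate X, Y and Z outputs.
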(fn `RNGVector`
  (params (InVector :type "Vector Structure") (InMin :type "Float (double-precision)") (InMax :type "Float (double-precision)"))
  (returns (Result :type "Vector Structure"))
  (bind (_invector_x _invector_y _invector_z) (`KismetMathLibrary.BreakVector` (`local.InVector`)))
  (return (`KismetMathLibrary.MakeVector` (* _invector_x (`KismetMathLibrary.RandomFloatInRange` (`local.InMin`) (`local.InMax`))) (* _invector_y (`KismetMathLibrary.RandomFloatInRange` (`local.InMin`) (`local.InMax`))) (* _invector_z (`KismetMathLibrary.RandomFloatInRange` (`local.InMin`) (`local.InMax`))))))