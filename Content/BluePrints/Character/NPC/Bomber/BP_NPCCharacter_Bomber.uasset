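; Bomber NPC character that arms itself when badly hurt and spawns explosions.
; Damage is routed to the main stats component, then an HP check at just under half health switches behavior, makes the mesh glow and plays a siren.
; Once armed, Tick spawns an explosion actor through a repeating five-second Delay without destroying the character itself.
; Destruction of the actor also spawns an explosion.
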(event `self.ReceiveBeginPlay`
  (`parent.ReceiveBeginPlay`)
  (bind _returnvalue (`PrimitiveComponent.CreateDynamicMaterialInstance` (`self.Mesh`) 0 null "None"))
  (set `self.M_Refference` _returnvalue))

(event `self.ReceiveAnyDamage`
  (params (Damage :type "Float (single-precision)") (DamageType :type "DamageType Object Reference") (InstigatedBy :type "Controller Object Reference") (DamageCauser :type "Actor Object Reference"))
  (bind _asbp_damage_object (cast `/Game/BluePrints/Objects/BP_DamageObject` DamageType))
  (`/Game/BluePrints/Components/BP_MainStatsComponent.ReceiveDamage` (`self.BP_MainStatsComponent`) Damage (`/Game/BluePrints/Objects/BP_DamageObject.DamageType` _asbp_damage_object) DamageCauser)
  (`self.CheckLowHP`))

(event `self.ReceiveDestroyed`
  (`self.SpawnBomb`))

(event `self.ReceiveTick`
  (params (DeltaSeconds :type "Float (single-precision)"))
  (`parent.ReceiveTick` DeltaSeconds)
  (if (`self.BomberActivate`)
    (`KismetSystemLibrary.Delay` 5.0)
    (`self.SpawnBomb`)))

(fn `BomberUpdateBehaviour`
  (params (BomberActivate :type Boolean))
  (if BomberActivate
    (set `/Game/BluePrints/Components/BP_MainStatsComponent.CurrentBehavor` "NewEnumerator3" (`self.BP_MainStatsComponent`))
    (`MaterialInstanceDynamic.SetScalarParameterValue` (`self.M_Refference`) "GlowParametr" 5.0)
    (`AudioComponent.Play` (`self.AudioSiren`) 0.0)))

(fn `CheckLowHP`
  (set `self.CurrentHPProgress` (`KismetMathLibrary.MapRangeClamped` (`KismetMathLibrary.Conv_IntToDouble` (`/Game/BluePrints/Components/BP_MainStatsComponent.CurrentHP` (`self.BP_MainStatsComponent`))) 0.0 (`KismetMathLibrary.Conv_IntToDouble` (`.MaxHP_11_D01976AF44B7651B89501589ACFCB2C6` (break `/Game/BluePrints/Structures/STRUCT_MainStats` (`/Game/BluePrints/Components/BP_MainStatsComponent.MainStatsStructure` (`self.BP_MainStatsComponent`))))) 0.0 1.0))
  (if (<= (`self.CurrentHPProgress`) 0.49)
    (bind _output_get (set `self.BomberActivate` true))
    (`self.BomberUpdateBehaviour` _output_get)))

(fn `DeadBomber`
  (`self.K2_DestroyActor`))

(fn `SpawnBomb`
  (`|SpawnActorFromClass` "/Game/BluePrints/Weapons/Projectiles/BP_Explossion_Bomber.BP_Explossion_Bomber_C" (`self.GetTransform`) "AlwaysSpawn" "OverrideRootScale" self null))

(fn `UserConstructionScript`
  (`parent.UserConstructionScript`))