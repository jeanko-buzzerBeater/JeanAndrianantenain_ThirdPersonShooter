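; BP_NPCCharacter_DD_A is an NPC character variant that adds weapon aiming on top of its parent class.
; Its UpdateWeaponSceneRotation override runs the parent logic, then acts only while the current weapon is shooting and BP_AIController is chasing a valid target.
; It smoothly interpolates WeaponScene's world pitch and yaw toward the target character's location, forcing roll to zero.
; The event graph and construction script add no logic of their own.
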(fn `UpdateWeaponSceneRotation`
  (locals (L_TargetLocation :type "Vector Structure" :default (0.0 0.0 0.0)))
  (`parent.UpdateWeaponSceneRotation`)
  (bind _currentweapon (`self.CurrentWeapon`)
    (:`then`
      (switch `/Game/BluePrints/Enum/ENUM_WeaponState` (`/Game/BluePrints/Weapons/BP_WeaponBase.WeaponState` _currentweapon)
        (:`NewEnumerator1`
          (bind _asbp_aicontroller (cast `/Game/BluePrints/Controllers/BP_AIController` (`self.GetController`)))
          (switch `/Game/BluePrints/Enum/ENUM_AIStates` (`/Game/BluePrints/Controllers/BP_AIController.AIState` _asbp_aicontroller)
            (:`NewEnumerator3`
              (bind _targetcharacter (`/Game/BluePrints/Controllers/BP_AIController.TargetCharacter` _asbp_aicontroller)
                (:`then`
                  (set `local.L_TargetLocation` (`self.K2_GetActorLocation` _targetcharacter))
                  (`SceneComponent.K2_SetWorldRotation` (`self.WeaponScene`) (`KismetMathLibrary.MakeRotator` 0.0 (.pitch (`KismetMathLibrary.RInterpTo` (`SceneComponent.K2_GetComponentRotation` (`self.WeaponScene`)) (`KismetMathLibrary.FindLookAtRotation` (`SceneComponent.K2_GetComponentLocation` (`self.WeaponScene`)) (`local.L_TargetLocation`)) (`GameplayStatics.GetWorldDeltaSeconds`) 10.0)) (.yaw (`KismetMathLibrary.RInterpTo` (`SceneComponent.K2_GetComponentRotation` (`self.WeaponScene`)) (`KismetMathLibrary.FindLookAtRotation` (`SceneComponent.K2_GetComponentLocation` (`self.WeaponScene`)) (`local.L_TargetLocation`)) (`GameplayStatics.GetWorldDeltaSeconds`) 10.0))) false false))
                (:`else`)))))))
    (:`else`)))

(fn `UserConstructionScript`
  (`parent.UserConstructionScript`))