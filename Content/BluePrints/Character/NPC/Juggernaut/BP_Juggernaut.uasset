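; Juggernaut NPC Blueprint that changes its weapon loadout and behavior when its health drops below about half.
; On BeginPlay it has the backpack weapon component spawn a shotgun-first, rifle-second loadout.
; Tick polls HP from the main stats component, switching the behavior enum while low.
; The first low-HP check also respawns the weapons in reversed order, latched by a flag so the swap happens only once.
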(event `self.ReceiveBeginPlay`
  (`parent.ReceiveBeginPlay`)
  (`self.StartGun`)
  (`/Game/BluePrints/Components/BP_Backpack_Weapon_Component.CheckAndSpawnWeapon` (`self.BP_Backpack_Weapon_Component`) (`self.FirstWeaponJug`) (`self.Second Weapon`)))

(event `self.ReceiveTick`
  (params (DeltaSeconds :type "Float (single-precision)"))
  (`parent.ReceiveTick` DeltaSeconds)
  (bind _checkswapweapon (`self.CheckLowHP`))
  (`self.SwitchWeapons` _checkswapweapon)
  (if (`self.SwapWeapon`)
    (set `/Game/BluePrints/Components/BP_MainStatsComponent.CurrentBehavor` "NewEnumerator2" (`self.BP_MainStatsComponent`))))

(fn `CheckLowHP`
  (returns (CheckSwapWeapon :type Boolean))
  (set `self.CurrentHPProgress` (`KismetMathLibrary.MapRangeClamped` (`KismetMathLibrary.Conv_IntToDouble` (`/Game/BluePrints/Components/BP_MainStatsComponent.CurrentHP` (`self.BP_MainStatsComponent`))) 0.0 (`KismetMathLibrary.Conv_IntToDouble` (`.MaxHP_11_D01976AF44B7651B89501589ACFCB2C6` (break `/Game/BluePrints/Structures/STRUCT_MainStats` (`/Game/BluePrints/Components/BP_MainStatsComponent.MainStatsStructure` (`self.BP_MainStatsComponent`))))) 0.0 1.0))
  (if (<= (`self.CurrentHPProgress`) 0.49)
    (set `self.SwapWeapon` true)
    (else
      (set `self.SwapWeapon` false)))
  (return (`self.SwapWeapon`)))

(fn `InEndSwapWeaponUpdated`
  (params (InFirstWeaponJug :type Name) (InSecondWeaponJug :type Name))
  (`/Game/BluePrints/Components/BP_Backpack_Weapon_Component.CheckAndSpawnWeapon` (`self.BP_Backpack_Weapon_Component`) InFirstWeaponJug InSecondWeaponJug)
  (set `self.InEndSwapWeapon` true))

(fn `StartGun`
  (set `self.FirstWeaponJug` "Shotgun_A")
  (set `self.Second Weapon` "Rifle_A"))

(fn `SwitchWeapons`
  (params (CheckSwapWeapons :type Boolean))
  (locals (L_FirstWeapon :type Name :default "None") (L_SecondWeapon :type Name :default "None"))
  (if (`local.CheckSwapWeapons`)
    (set `self.FirstWeaponJug` "Rifle_A")
    (set `self.Second Weapon` "Shotgun_A")
    (if (not (`self.InEndSwapWeapon`))
      (`self.InEndSwapWeaponUpdated` (`self.FirstWeaponJug`) (`self.Second Weapon`)))))

(fn `UserConstructionScript`
  (`parent.UserConstructionScript`))