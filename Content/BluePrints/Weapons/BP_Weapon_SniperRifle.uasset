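; Sniper rifle weapon, a child Blueprint that replaces the parent's single shot with a long-range hitscan and adds an aim laser.
; SingleShot line-traces from the muzzle with debug drawing left on, then plays shot effects.
; Hits apply a physics impulse (radial force for non-simulating components, meant for destructibles), damage tripled on the "head" bone, and an attached impact actor.
; Tick traces the laser, scaling its beam mesh and moving a point light to the hit.
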(event `self.ReceiveBeginPlay`
  (`parent.ReceiveBeginPlay`)
  (`self.AimLaserConfigure`))

(event `self.ReceiveTick`
  (params (DeltaSeconds :type "Float (single-precision)"))
  (`parent.ReceiveTick` DeltaSeconds)
  (`self.AimLaserUpdate`))

(fn `AddPhusicsImpuls`
  (bind _hitcomponent (`self.HitComponent`)
    (:`then`
      (if (`SceneComponent.IsSimulatingPhysics` _hitcomponent "None")
        (`PrimitiveComponent.AddImpulseAtLocation` (`self.HitComponent`) (* (* (`KismetMathLibrary.Normal` (- (`self.HitLocation`) (`SceneComponent.K2_GetComponentLocation` (`self.MuzzleScene`)))) 2000.0) (`self.ImpulsMult`)) (`self.HitLocation`) "None")
        (else
          ;[1 0.8636 0] Warning! Only for Destructibles
          (`SceneComponent.K2_SetWorldLocation` (`self.RadialForce`) (`self.HitLocation`) false false)
          (`RadialForceComponent.FireImpulse` (`self.RadialForce`)))))
    (:`else`)))

(fn `AimLaserConfigure`
  (`StaticMeshComponent.SetStaticMesh` (`self.AimLaserStaticMesh`) (`self.AimSm`))
  (`PrimitiveComponent.SetMaterial` (`self.AimLaserStaticMesh`) 0 (`self.AImMI`)))

(fn `AimLaserUpdate`
  (locals (L_Dist :type "Float (double-precision)" :default 0.0) (L_Loc :type "Vector Structure" :default (0.0 0.0 0.0)))
  (bind _aimlaser (`self.AimLaser`))
  (bind _aimlaserstaticmesh (`self.AimLaserStaticMesh`))
  (bind _returnvalue (`SceneComponent.K2_GetComponentLocation` _aimlaser))
  (bind (_returnvalue_x _returnvalue_y _returnvalue_z) (`KismetMathLibrary.BreakVector` (`SceneComponent.K2_GetComponentScale` _aimlaserstaticmesh)))
  (bind (_returnvalue_x_2 _returnvalue_y_2 _returnvalue_z_2) (`KismetMathLibrary.BreakVector` (`SceneComponent.K2_GetComponentScale` (`self.AimLaserStaticMesh`))))
  (bind (_outhit _returnvalue_2) (`KismetSystemLibrary.LineTraceSingle` _returnvalue (+ _returnvalue (* (`SceneComponent.GetForwardVector` _aimlaser) 5000.0)) "TraceTypeQuery2" true))
  (if _returnvalue_2
    (bind (_bblockinghit _binitialoverlap _time _distance _location) (`GameplayStatics.BreakHitResult` _outhit))
    (set `local.L_Dist` _distance)
    (set `local.L_Loc` _location)
    (`SceneComponent.SetWorldScale3D` (`self.AimLaserStaticMesh`) (`KismetMathLibrary.MakeVector` (/ (`local.L_Dist`) 1000.0) _returnvalue_y_2 _returnvalue_z_2))
    (`SceneComponent.K2_SetWorldLocation` (`self.AimLaserPoinLight`) (`local.L_Loc`) false false)
    (`LightComponent.SetIntensity` (`self.AimLaserPoinLight`) 1000.0)
    (else
      (`SceneComponent.SetWorldScale3D` _aimlaserstaticmesh (`KismetMathLibrary.MakeVector` 1.0 _returnvalue_y _returnvalue_z))
      (`SceneComponent.K2_SetWorldLocation` (`self.AimLaserPoinLight`) (`SceneComponent.K2_GetComponentLocation` (`self.AimLaser`)) false false)
      (`LightComponent.SetIntensity` (`self.AimLaserPoinLight`) (`self.AimLightIntencity`)))))

(fn `ApplyDamageByHitscan`
  (locals (L_Damage :type Integer :default 0))
  (`|ExecutionSequence`
    (:`then_0`
      (set `local.L_Damage` 100))
    (:`then_1`
      (if (== (`.HitBoneName` (`GameplayStatics.BreakHitResult` (`self.HitResult`))) "head")
        (set `local.L_Damage` (* (`local.L_Damage`) 3))))
    (:`then_2`
      (`GameplayStatics.ApplyDamage` (`self.HitActor`) (`KismetMathLibrary.Conv_IntToDouble` (`local.L_Damage`)) null (`self.GetOwner`) "/Game/BluePrints/Objects/BP_DamageObject.BP_DamageObject_C"))))

(fn `Configure Weapon Stats`
  (params (InWeaponName :type Name))
  (`parent.Configure Weapon Stats` InWeaponName)
  (`SkinnedMeshComponent.SetSkinnedAssetAndUpdate` (`self.SkeletalMesh`) null true))

(fn `SingleShot`
  (bind (_bblockinghit _binitialoverlap _time _distance _location _impactpoint _normal _impactnormal _physmat _hitactor _hitcomponent) (`GameplayStatics.BreakHitResult` (`self.HitResult`)))
  (bind _returnvalue (`SceneComponent.K2_GetComponentLocation` (`self.MuzzleScene`)))
  (`|ExecutionSequence`
    (:`then_0`
      (bind (_outhit _returnvalue_2) (`KismetSystemLibrary.LineTraceSingle` _returnvalue (+ _returnvalue (* (`SceneComponent.GetForwardVector` (`self.MuzzleScene`)) 25000.0)) "TraceTypeQuery2" true (`|MakeArray` self (`self.GetOwner`) :!type "Actor Object Reference") "ForDuration" true (struct :`R` 1.0 :`A` 1.0) (struct :`G` 1.0 :`A` 1.0) 10.0))
      (if _returnvalue_2
        (set `self.HitResult` _outhit)
        (set `self.HitLocation` _location)
        (set `self.HitNormal` _normal)
        (set `self.HitActor` _hitactor)
        (set `self.HitComponent` _hitcomponent)
        (`|ExecutionSequence`
          (:`then_0`
            (`self.AddPhusicsImpuls`))
          (:`then_1`
            (`self.ApplyDamageByHitscan`))
          (:`then_2`
            (`self.SpawnDecal`)))))
    (:`then_1`
      (`self.ShotEffects`))))

(fn `SpawnDecal`
  (locals (L_Rotator :type "Rotator Structure" :default (struct)) (L_Impact :type "/Game/BluePrints/Weapons/Projectiles/BP_ImpactEffect Object Reference"))
  (bind (_returnvalue_roll _returnvalue_pitch _returnvalue_yaw) (`KismetMathLibrary.BreakRotator` (`KismetMathLibrary.Conv_VectorToRotator` (`self.HitNormal`))))
  (set `local.L_Rotator` (`KismetMathLibrary.MakeRotator` (`KismetMathLibrary.RandomFloatInRange` 0.0 360.0) _returnvalue_pitch _returnvalue_yaw))
  (bind _returnvalue (`|SpawnActorFromClass` "/Game/BluePrints/Weapons/Projectiles/BP_ImpactEffect.BP_ImpactEffect_C" (`KismetMathLibrary.MakeTransform` (`self.HitLocation`) (`local.L_Rotator`)) "Undefined" "OverrideRootScale" self null))
  (set `local.L_Impact` _returnvalue)
  (`self.K2_AttachToComponent` (`local.L_Impact`) (`self.HitComponent`) (`.HitBoneName` (`GameplayStatics.BreakHitResult` (`self.HitResult`))) "KeepWorld" "KeepWorld" "KeepWorld" true))

(fn `UserConstructionScript`
  (`parent.UserConstructionScript`))