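; BP_Item_Weapon is a weapon pickup item that a character collects into their weapon backpack.
; Interact checks that the item is ready and the character in its box has a BP_Backpack_Weapon_Component, then calls PutIntoBackpack, returning true on every path.
; PutIntoBackpack runs the parent logic, then for a named item either adds the weapon or uses the full-backpack call when both slots are filled, and finishes with AfterUse.
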(fn `Interact`
  (returns (Success :type Boolean))
  (if (`self.IsReadeToInteract`)
    (bind _characterinbox (`self.CharacterInBox`)
      (:`then`
        (bind _returnvalue (`self.GetComponentByClass` _characterinbox "/Game/BluePrints/Components/BP_Backpack_Weapon_Component.BP_Backpack_Weapon_Component_C"))
        (`/Engine/EditorBlueprintResources/StandardMacros.IsValid` _returnvalue
          (:`Is Valid`
            (`self.PutIntoBackpack` null _returnvalue)
            (return true))
          (:`Is Not Valid`
            (return true))))
      (:`else`
        (return true)))
    (else
      (return true))))

(fn `PutIntoBackpack`
  (params (InBackpack :type "/Game/BluePrints/Components/BP_BackpackComponent Object Reference") (InBackPackWeapons :type "/Game/BluePrints/Components/BP_Backpack_Weapon_Component Object Reference"))
  (locals (L_Backpack :type "/Game/BluePrints/Components/BP_BackpackComponent Object Reference") (L_BackpackWeapon :type "/Game/BluePrints/Components/BP_Backpack_Weapon_Component Object Reference") (L_AvalableWeaponNames :type "Array of Name") (WeaponIndexItem :type Integer :default 0))
  (bind _output_get (set `local.L_BackpackWeapon` InBackPackWeapons))
  (`parent.PutIntoBackpack` null _output_get)
  (if (!= (`self.ItemName`) "None")
    (`|ExecutionSequence`
      (:`then_0`
        (if (!= (`/Game/BluePrints/Components/BP_Backpack_Weapon_Component.FirstWeapon` (`local.L_BackpackWeapon`)) "None")
          (if (!= (`/Game/BluePrints/Components/BP_Backpack_Weapon_Component.SecondWeapon` (`local.L_BackpackWeapon`)) "None")
            (`/Game/BluePrints/Components/BP_Backpack_Weapon_Component.AddWeaponFullBackpack` (`local.L_BackpackWeapon`) (`self.ItemName`))
            (else
              (`/Game/BluePrints/Components/BP_Backpack_Weapon_Component.AddWeaponItem` (`local.L_BackpackWeapon`) (`self.ItemName`))))
          (else
            (`/Game/BluePrints/Components/BP_Backpack_Weapon_Component.AddWeaponItem` (`local.L_BackpackWeapon`) (`self.ItemName`)))))
      (:`then_1`
        (`self.AfterUse`)))))

(fn `UserConstructionScript`
  (`parent.UserConstructionScript`))