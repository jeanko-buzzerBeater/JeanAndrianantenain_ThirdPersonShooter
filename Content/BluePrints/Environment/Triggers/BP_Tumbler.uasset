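; Toggle switch actor that flips the lock on its assigned doors when interacted with inside its overlap area, where it also shows a text prompt.
; Interact calls SwitchOn or SwitchOff, playing a timeline forward or backward to slide the stick, with InProgress blocking re-triggers.
; When the timeline finishes, it updates the state, calls SwitchLock on each door and fires OnDoorsLockSwitched.
; The construction script offsets the stick to match the initial state.
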(event `self.ReceiveBeginPlay`
  (`SceneComponent.SetVisibility` (`self.TextRender`) false false))

(event `self.ReceiveActorBeginOverlap`
  (params (OtherActor :type "Actor Object Reference"))
  (`SceneComponent.SetVisibility` (`self.TextRender`) true false)
  (set `self.IsReadeToInteract` true))

(event `self.ReceiveActorEndOverlap`
  (params (OtherActor :type "Actor Object Reference"))
  (`SceneComponent.SetVisibility` (`self.TextRender`) false false)
  (set `self.IsReadeToInteract` false))

(event `SwitchOn`
  (if (not (`self.InProgress`))
    (if (not (`self.IsTumblerOn`))
      (bind (_direction _move) (`Timeline|TumblerTimeLine` :!via `PlayFromStart` :!label _label)
        (:`Update`
          (set `self.InProgress` true)
          (`SceneComponent.K2_SetRelativeLocation` (`self.TumblerStickMesh`) (`KismetMathLibrary.MakeVector` 0.0 (* (`self.MaxStickOffset`) _move)) false false))
        (:`Finished`
          (set `self.InProgress` false)
          (switch `ETimelineDirection` _direction
            (:`Forward`
              (set `self.IsTumblerOn` true))
            (:`Backward`
              (set `self.IsTumblerOn` false)))
          (`self.DoorsLockSwitch`)
          (`self.OnDoorsLockSwitched` (`self.IsTumblerOn`)))))))

(event `SwitchOff`
  (if (not (`self.InProgress`))
    (if (`self.IsTumblerOn`)
      (goto _label :!via `ReverseFromEnd`))))

(fn `DoorsLockSwitch`
  (if (`KismetArrayLibrary.Array_IsValidIndex` (`self.DoorsToLockSwitch`))
    (for _array_element (`self.DoorsToLockSwitch`)
      (`/Game/BluePrints/Environment/Doors/BP_Door_WithLock.SwitchLock` _array_element))))

(fn `Interact`
  (returns (Success :type Boolean))
  (if (`self.IsReadeToInteract`)
    (if (`self.IsTumblerOn`)
      (`self.SwitchOff`)
      (return true)
      (else
        (`self.SwitchOn`)
        (return true)))
    (else
      (return false))))

(fn `UserConstructionScript`
  (`SceneComponent.K2_AddRelativeLocation` (`self.TumblerStickMesh`) (`KismetMathLibrary.MakeVector` 0.0 (`KismetMathLibrary.SelectFloat` (`self.MaxStickOffset`) 0.0 (`self.IsTumblerOn`))) false false))