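; BP_Tooltip_LookOn is a tooltip actor whose TooltipText turns to face the player's camera.
; Actor overlap sets a LookAt flag when PlayerInBox is valid, and any end overlap clears it.
; While the flag is set, Tick rotates the text each frame toward the BP_PlayerCharacter camera using FindLookAtRotation.
; Tick and overlap events call their parent versions first, and PlayerInBox is not assigned here.
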(event `self.ReceiveTick`
  (params (DeltaSeconds :type "Float (single-precision)"))
  (`parent.ReceiveTick` DeltaSeconds)
  (`self.LookingAtPlayerCamera`))

(event `self.ReceiveActorBeginOverlap`
  (params (OtherActor :type "Actor Object Reference"))
  (`parent.ReceiveActorBeginOverlap` OtherActor)
  (`self.PlayerInBox`
    (:`then`
      (set `self.LookAt` true))
    (:`else`)))

(event `self.ReceiveActorEndOverlap`
  (params (OtherActor :type "Actor Object Reference"))
  (`parent.ReceiveActorEndOverlap` OtherActor)
  (set `self.LookAt` false))

(fn `LookingAtPlayerCamera`
  (locals (L_CameraLocation :type "Vector Structure" :default (0.0 0.0 0.0)))
  (if (`self.LookAt`)
    (bind _playerinbox (`self.PlayerInBox`)
      (:`then`
        (bind _asbp_player_character (cast `/Game/BluePrints/Character/Player/BP_PlayerCharacter` _playerinbox))
        (set `local.L_CameraLocation` (`SceneComponent.K2_GetComponentLocation` (`/Game/BluePrints/Character/Player/BP_PlayerCharacter.Camera` _asbp_player_character)))
        (`SceneComponent.K2_SetWorldRotation` (`self.TooltipText`) (`KismetMathLibrary.FindLookAtRotation` (`SceneComponent.K2_GetComponentLocation` (`self.TooltipText`)) (`local.L_CameraLocation`)) false false))
      (:`else`))))

(fn `UserConstructionScript`
  (`parent.UserConstructionScript`))